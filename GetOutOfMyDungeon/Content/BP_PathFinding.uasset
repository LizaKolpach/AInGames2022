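; A* pathfinder over linked grid tiles that finds routes weighted per enemy type.
; FindPath costs each step by the tile's EnemyValue and returns the start-to-goal tile array, while HasPathToGoal only checks reachability using unit costs.
; Both pick the lowest length-plus-heuristic open tile by linear array scans.
; The heuristic is floored Euclidean grid distance, scaled by the averaged enemy value of both endpoints when a name is given.
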(fn `FindNextOpen`
  (params (OpenArray :type "Array of /Game/BP_PathFindingNode Object Reference") (DataArray :type "Array of /Game/STRUCT_NodeLink Structure"))
  (returns (Return :type "/Game/BP_PathFindingNode Object Reference") (index :type Integer))
  (locals (Length :type Integer :default 2147483647) (ArrIndex :type Integer) (ReturnVal :type "/Game/BP_PathFindingNode Object Reference"))
  ;[1 1 1] Find the smallest return value (heuristic + path length)
  (for (_array_element _array_index) OpenArray
    (for _array_element_2 DataArray
      (bind (_self _parent _heuristic _pathlength) (break `/Game/STRUCT_NodeLink` _array_element_2))
      (if (== _self _array_element)
        (bind _returnvalue (+ _pathlength _heuristic))
        (if (< _returnvalue (`local.Length`))
          (set `local.Length` _returnvalue)
          (set `local.ReturnVal` _array_element)
          (set `local.ArrIndex` _array_index)
          (break)))))
  (return (`local.ReturnVal`) (`local.ArrIndex`)))

(fn `FindPath`
  (params (Start :type "/Game/BP_PathFindingNode Object Reference") (Goal :type "/Game/BP_PathFindingNode Object Reference") (EnemyName :type Name))
  (returns (FinalPath :type "Array of /Game/BP_PathFindingNode Object Reference") (FoundPath :type Boolean))
  (locals (Path :type "Array of /Game/STRUCT_NodeLink Structure") (Open :type "Array of /Game/BP_PathFindingNode Object Reference") (EndGoal :type "/Game/BP_PathFindingNode Object Reference") (Index :type Integer) (Next :type "/Game/BP_PathFindingNode Object Reference") (Neighbour :type "/Game/BP_PathFindingNode Object Reference") (Enemy :type Name) (FinalArr :type "Array of /Game/BP_PathFindingNode Object Reference") (HasParent :type Boolean))
  (bind _open (`local.Open`))
  (bind _enemy (`local.Enemy`))
  (bind _neighbour (`local.Neighbour`))
  (bind _next (`local.Next`))
  (set `local.Enemy` EnemyName)
  ;[1 0 0.04771] Big Fucking TODO: structs are unreliable and need proper testing to see if they work
  ;;[1 1 1] Add the intitial start to the list
  (set `local.EndGoal` Goal)
  (bind _heuristics (`self.GetHeuristics` Start (`local.EndGoal`) (`local.Enemy`)))
  (`KismetArrayLibrary.Array_Add` (`local.Path`) (make `/Game/STRUCT_NodeLink` Start null _heuristics 1))
  (`KismetArrayLibrary.Array_AddUnique` _open Start)
  ;;[1 1 1] If there are no open places left then it couldnt find the end
  (while (> (`KismetArrayLibrary.Array_Length` _open) 0)
    ;;[1 1 1] Get the closest next item and remove it from the open list
    (bind _return (`self.FindNextOpen` (`local.Open`) (`local.Path`)))
    (bind _output_get (set `local.Next` _return))
    (`KismetArrayLibrary.Array_RemoveItem` (`local.Open`) _output_get)
    ;;[1 1 1] If that next item is the end then we start creating the path
    (if (== (`local.Next`) (`local.EndGoal`))
      (bind _data (`self.FindPathData` (`local.Next`) (`local.Path`)))
      ;;[1 1 1] While next has a parent add it to the array
      (while (`local.HasParent`)
        (`KismetArrayLibrary.Array_Add` (`local.FinalArr`) _next)
        (bind _data_2 (`self.FindPathData` _next (`local.Path`)))
        (set `local.Next` (`.Parent_14_4C838F96427D2ED138DCC89C6AE0275D` (break `/Game/STRUCT_NodeLink` _data_2)))
        (set `local.HasParent` (`KismetSystemLibrary.IsValid` (`.Parent_14_4C838F96427D2ED138DCC89C6AE0275D` (break `/Game/STRUCT_NodeLink` _data_2)))))
      ;;[1 1 1] Make sure to add the starting point aswell
      (`KismetArrayLibrary.Array_Add` (`local.FinalArr`) (`local.Next`))
      ;;[1 1 1] Reverse order so the start is at the front
      (`KismetArrayLibrary.Array_Reverse` (`local.FinalArr`))
      (return (`local.FinalArr`) true)
      (else
        ;;[1 1 1] Get the next path data
        (bind _data_3 (`self.FindPathData` (`local.Next`) (`local.Path`)))
        (set `local.Index` (`.PathLength_13_AAE0EFCC43222E75278BB09E7635CED6` (break `/Game/STRUCT_NodeLink` _data_3)))
        ;;[1 1 1] Loop over all the neigbours
        (for _array_element (`/Game/BP_PathFindingNode.Neighbours` (`local.Next`))
          (set `local.Neighbour` _array_element)
          ;;[1 1 1] See if if the neigbour has already been found
          (bind (_data_4 _array_index) (`self.FindPathData` (`local.Neighbour`) (`local.Path`)))
          (bind (_self _parent _heuristic _pathlength) (break `/Game/STRUCT_NodeLink` _data_4))
          (`/Engine/EditorBlueprintResources/StandardMacros.IsValid` _self
            (:`Is Valid`
              (bind _returnvalue (+ (`local.Index`) (`self.FindWeight` (`local.Enemy`) _self)))
              ;;[1 1 1] If the new path is smaller then the one already recorded change it
              (if (< _returnvalue _pathlength)
                (bind _heuristics_2 (`self.GetHeuristics` _self (`local.EndGoal`) (`local.Enemy`)))
                (`KismetArrayLibrary.Array_Insert` (`local.Path`) (make `/Game/STRUCT_NodeLink` _self (`local.Next`) _heuristics_2 _returnvalue) _array_index)
                ;[1 1 1] Add this neigbour to the open list
                (`KismetArrayLibrary.Array_Add` (`local.Open`) (`local.Neighbour`) :!label _label)))
            (:`Is Not Valid`
              ;;[1 1 1] Add a new open path
              (bind _heuristics_3 (`self.GetHeuristics` _neighbour (`local.EndGoal`) _enemy))
              (`KismetArrayLibrary.Array_Add` (`local.Path`) (make `/Game/STRUCT_NodeLink` _neighbour (`local.Next`) _heuristics_3 (+ (`local.Index`) (`self.FindWeight` _enemy (`local.Neighbour`)))))
              (goto _label)))))))
  (return _ false))

(fn `FindPathData`
  (params (Item :type "/Game/BP_PathFindingNode Object Reference") (DataArray :type "Array of /Game/STRUCT_NodeLink Structure"))
  (returns (Data :type "/Game/STRUCT_NodeLink Structure") (`Array Index` :type Integer))
  ;[1 1 1] Find the correct data that fits the item
  (for (_array_element _array_index) DataArray
    (if (== (`.Self_7_6BCF11FB47FDBD09122A3EBE29D34417` (break `/Game/STRUCT_NodeLink` _array_element)) Item)
      (return _array_element _array_index)))
  (return (struct) -1))

(fn `FindWeight`
  (params (Enemy :type Name) (Tile :type "/Game/BP_PathFindingNode Object Reference"))
  (returns (Value :type Integer))
  (return (`BlueprintMapLibrary.Map_Find` (`/Game/BP_PathFindingNode.EnemyValue` Tile) Enemy)))

(fn `GetHeuristics`
  (params (Start :type "/Game/BP_PathFindingNode Object Reference") (End :type "/Game/BP_PathFindingNode Object Reference") (Name :type Name :default "None"))
  (returns (Heuristics :type Integer))
  (locals (Multiplier :type Integer))
  (bind _returnvalue (- (`/Game/BP_PathFindingNode.GridPositionX` End) (`/Game/BP_PathFindingNode.GridPositionX` Start)))
  (bind _returnvalue_2 (- (`/Game/BP_PathFindingNode.GridPositionY` End) (`/Game/BP_PathFindingNode.GridPositionY` Start)))
  ;[1 1 1] Get the right multiplier(takes average of start and end to calculate it), if no input then 1 will be asumed
  (if (== Name "None")
    (set `local.Multiplier` 1)
    (else
      (set `local.Multiplier` (/ (+ (`BlueprintMapLibrary.Map_Find` (`/Game/BP_PathFindingNode.EnemyValue` Start) Name) (`BlueprintMapLibrary.Map_Find` (`/Game/BP_PathFindingNode.EnemyValue` End) Name)) 2))))
  (return (* (`KismetMathLibrary.FFloor` (`KismetMathLibrary.Sqrt` (`KismetMathLibrary.Conv_IntToDouble` (+ (* _returnvalue _returnvalue) (* _returnvalue_2 _returnvalue_2))))) (`local.Multiplier`))))

(fn `HasPathToGoal`
  (params (Start :type "/Game/BP_PathFindingNode Object Reference") (Goal :type "/Game/BP_PathFindingNode Object Reference"))
  (returns (HasPath :type Boolean))
  (locals (Path :type "Array of /Game/STRUCT_NodeLink Structure") (Open :type "Array of /Game/BP_PathFindingNode Object Reference") (EndGoal :type "/Game/BP_PathFindingNode Object Reference") (Index :type Integer) (Next :type "/Game/BP_PathFindingNode Object Reference") (Neighbour :type "/Game/BP_PathFindingNode Object Reference"))
  (bind _open (`local.Open`))
  (bind _neighbour (`local.Neighbour`))
  (bind _returnvalue (+ (`local.Index`) 1))
  ;[1 0 0.04771] Big Fucking TODO: structs are unreliable and need proper testing to see if they work
  ;;[1 1 1] Add the intitial start to the list
  (set `local.EndGoal` Goal)
  (bind _heuristics (`self.GetHeuristics` Start (`local.EndGoal`)))
  (`KismetArrayLibrary.Array_Add` (`local.Path`) (make `/Game/STRUCT_NodeLink` Start null _heuristics 1))
  (`KismetArrayLibrary.Array_AddUnique` _open Start)
  ;;[1 1 1] If there are no open places left then it couldnt find the end
  (while (> (`KismetArrayLibrary.Array_Length` _open) 0)
    ;;[1 1 1] Get the closest next item and remove it from the open list
    (bind _return (`self.FindNextOpen` (`local.Open`) (`local.Path`)))
    (bind _output_get (set `local.Next` _return))
    (`KismetArrayLibrary.Array_RemoveItem` (`local.Open`) _output_get)
    ;;[1 1 1] If that next item is the end then we found the solution
    (if (== (`local.Next`) (`local.EndGoal`))
      (return true)
      (else
        ;;[1 1 1] Get the next path data
        (bind _data (`self.FindPathData` (`local.Next`) (`local.Path`)))
        (set `local.Index` (`.PathLength_13_AAE0EFCC43222E75278BB09E7635CED6` (break `/Game/STRUCT_NodeLink` _data)))
        ;;[1 1 1] Loop over all the neigbours
        (for _array_element (`/Game/BP_PathFindingNode.Neighbours` (`local.Next`))
          (set `local.Neighbour` _array_element)
          ;;[1 1 1] See if if the neigbour has already been found
          (bind (_data_2 _array_index) (`self.FindPathData` (`local.Neighbour`) (`local.Path`)))
          (bind (_self _parent _heuristic _pathlength) (break `/Game/STRUCT_NodeLink` _data_2))
          (`/Engine/EditorBlueprintResources/StandardMacros.IsValid` _self
            (:`Is Valid`
              ;;[1 1 1] If the new path is smaller then the one already recorded change it
              (if (< _returnvalue _pathlength)
                (bind _heuristics_2 (`self.GetHeuristics` _self (`local.EndGoal`)))
                (`KismetArrayLibrary.Array_Insert` (`local.Path`) (make `/Game/STRUCT_NodeLink` _self (`local.Next`) _heuristics_2 _returnvalue) _array_index)
                ;[1 1 1] Add this neigbour to the open list
                (`KismetArrayLibrary.Array_Add` (`local.Open`) (`local.Neighbour`) :!label _label)))
            (:`Is Not Valid`
              ;;[1 1 1] Add a new open path
              (bind _heuristics_3 (`self.GetHeuristics` _neighbour (`local.EndGoal`)))
              (`KismetArrayLibrary.Array_Add` (`local.Path`) (make `/Game/STRUCT_NodeLink` _neighbour (`local.Next`) _heuristics_3 (+ (`local.Index`) 1)))
              (goto _label)))))))
  (return false))

(fn `UserConstructionScript`)