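; BP_RoomTest is a test room for grid-based placement that opens its walls where other rooms adjoin it.
; On BeginPlay it computes four neighbour grid positions from its location and the player controller's grid size, paired by index with four walls.
; CheckWalls hides and disables collision on walls facing occupied cells.
; A one-shot pass then asks neighbouring rooms to re-check, though it is commented as non-functional.
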(event `self.ReceiveBeginPlay`
  (bind (_gridlocation_x _gridlocation_y _gridlocation_z) (`KismetMathLibrary.BreakVector` (`self.GridLocation`)))
  (bind _gridsize (`/Game/GameJamGame/Blueprints/BP_PlayerController.GridSize` (`self.As BP Player Controller`)))
  (`parent.ReceiveBeginPlay`)
  ;[1 1 1] SaveNeighbourPositions
  (set `self.NeighbourNorth_0` (`KismetMathLibrary.MakeVector` (+ _gridlocation_x _gridsize) _gridlocation_y _gridlocation_z))
  (set `self.NeighbourSouth_0` (`KismetMathLibrary.MakeVector` (- _gridlocation_x _gridsize) _gridlocation_y _gridlocation_z))
  (set `self.NeighbourEast_0` (`KismetMathLibrary.MakeVector` _gridlocation_x (+ _gridlocation_y _gridsize) _gridlocation_z))
  (set `self.NeighbourWest_0` (`KismetMathLibrary.MakeVector` _gridlocation_x (- _gridlocation_y _gridsize) _gridlocation_z))
  ;[1 1 1] MakeArrays
  (`KismetArrayLibrary.Array_Clear` (`self.NeighbourArray_0_0`))
  (set `self.NeighbourArray_0_0` (`|MakeArray` (`self.NeighbourWest_0`) (`self.NeighbourEast_0`) (`self.NeighbourNorth_0`) (`self.NeighbourSouth_0`)))
  (set `self.WallArray_0` (`|MakeArray` (`self.WallW_0`) (`self.WallE_0`) (`self.WallN_0`) (`self.WallS_0`)))
  (`self.CheckWalls`))

(event `CheckWalls`
  ;[1 1 1] Remove walls if neighbours occupied
  (bind _asbp_player_controller (cast `/Game/GameJamGame/Blueprints/BP_PlayerController` (`GameplayStatics.GetPlayerController` 0)))
  (for (_array_element _array_index) (`self.NeighbourArray_0_0`)
    (if (`/Game/GameJamGame/Blueprints/BP_PlayerController.IsSelectedGridPositionOccupied` _asbp_player_controller _array_element)
      (bind _output (`|GetArrayItem` (`self.WallArray_0`) _array_index))
      (`SceneComponent.SetVisibility` _output false false)
      (`PrimitiveComponent.SetCollisionEnabled` _output "NoCollision")))
  ;[1 1 1] Non-functional: Have neighbours re-check their walls
  (`/Engine/EditorBlueprintResources/StandardMacros.DoOnce` false
    (:`Completed`
      (for _array_element_2 (`self.NeighbourArray_0_0`)
        (bind _asbp_room_test (cast `/Game/GameJamGame/EileenDev/BP_RoomTest` (`/Game/GameJamGame/Blueprints/BP_PlayerController.GetRoomAtSelectedGridPosition` _asbp_player_controller _array_element_2)))
        (`self.CheckWalls` _asbp_room_test)))))

(fn `UserConstructionScript`
  (`parent.UserConstructionScript`))