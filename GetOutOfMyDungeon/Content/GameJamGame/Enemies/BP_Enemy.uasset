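; BP_Enemy is an enemy actor for a dungeon game that tracks health and awards coins when killed.
; AnyDamage subtracts damage from clamped HP, prints it for debugging and spawns a damage particle effect.
; At zero HP, Death notifies GM_DungeonGameMode of the kill, adds a random coin amount to the first player controller's total, then destroys the actor.
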(event `self.ReceiveBeginPlay`
  (set `self.CurrentHP` (`self.MaxHP`)))

(event `self.ReceiveAnyDamage`
  (params (Damage :type "Float (single-precision)") (DamageType :type "DamageType Object Reference") (InstigatedBy :type "Controller Object Reference") (DamageCauser :type "Actor Object Reference"))
  (bind _output_get (set `self.CurrentHP` (`KismetMathLibrary.FClamp` (- (`self.CurrentHP`) Damage) 0.0 (`self.MaxHP`))))
  ;[1 0.07292 0.07292 1 15] remove for build
  (`KismetSystemLibrary.PrintString` (`KismetStringLibrary.Conv_DoubleToString` _output_get))
  (`NiagaraFunctionLibrary.SpawnSystemAtLocation` "/Game/GameJamGame/VFX/PS_DamageTaken.PS_DamageTaken" (`SceneComponent.K2_GetComponentLocation` (`self.ParticleLocation`)))
  (if (<= (`self.CurrentHP`) 0.0)
    (`self.Death`)))

(event `Death`
  (bind _asgm_dungeon_game_mode (cast `/Game/GameJamGame/Blueprints/GM_DungeonGameMode` (`GameplayStatics.GetGameMode`)))
  (`/Game/GameJamGame/Blueprints/GM_DungeonGameMode.EnemyKilled` _asgm_dungeon_game_mode)
  ;[1 1 1] connect the number from here to a player coin counter
  (`self.AddLootToPlayer`)
  (`self.K2_DestroyActor`))

(event `TEST_Move`)

(fn `AddLootToPlayer`
  (returns (CoinsAdded :type Integer))
  (bind _asbp_player_controller (cast `/Game/GameJamGame/Blueprints/BP_PlayerController` (`GameplayStatics.GetPlayerController` 0)))
  (bind _output_get (set `/Game/GameJamGame/Blueprints/BP_PlayerController.CurrentCoins` (+ (`/Game/GameJamGame/Blueprints/BP_PlayerController.CurrentCoins` _asbp_player_controller) (`KismetMathLibrary.RandomIntegerInRange` (`self.CoinsMin`) (`self.CoinsMax`))) _asbp_player_controller))
  (return _output_get))

(fn `UserConstructionScript`)