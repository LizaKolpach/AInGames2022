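; Player controller for grid-based room placement with the mouse.
; Each tick it traces under the cursor on the Camera channel, snaps the hit point to a 100-unit grid, prints it and draws a flat debug box as a cell preview.
; Left mouse click spawns a BP_Room at the snapped X and Y, leaving Z at default rather than using the hit height.
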(event `self.ReceiveTick`
  (params (DeltaSeconds :type "Float (single-precision)"))
  (bind _returnvalue (`KismetMathLibrary.Vector_SnappedToGrid` (`.ImpactPoint` (`GameplayStatics.BreakHitResult` (`self.GetHitResultUnderCursorByChannel` "TraceTypeQuery2"))) 100.0))
  (`KismetSystemLibrary.PrintString` (`KismetStringLibrary.Conv_VectorToString` _returnvalue) true true (struct :`G` 0.66 :`B` 1.0 :`A` 1.0) 0.0)
  (`KismetSystemLibrary.DrawDebugBox` _returnvalue (50.0 50.0 0.0) (struct :`R` 1.0 :`G` 0.084869 :`A` 1.0) (struct) 0.0 5.0))

(event `Key|LeftMouseButton`
  (params (Key :type "Key Structure"))
  (bind (_returnvalue_x _returnvalue_y) (`KismetMathLibrary.BreakVector` (`KismetMathLibrary.Vector_SnappedToGrid` (`.ImpactPoint` (`GameplayStatics.BreakHitResult` (`self.GetHitResultUnderCursorByChannel` "TraceTypeQuery2"))) 100.0)))
  (:`Pressed`
    (`|SpawnActorFromClass` "/Game/GameJamGame/DavyDev/BP_Room.BP_Room_C" (`KismetMathLibrary.MakeTransform` (`KismetMathLibrary.MakeVector` _returnvalue_x _returnvalue_y)) "Undefined" "OverrideRootScale" null null)))

(fn `UserConstructionScript`)