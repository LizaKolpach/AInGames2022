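; Game mode for a dungeon-building wave defense game, placing the enemy spawn and treasure rooms at BeginPlay through the player controller.
; StartWave refreshes room pathfinding and, if a route exists, computes separate Walker and Flyer paths via BP_PathFinding.
; It then reads the wave's DT_Waves row and spawns walkers, then flyers, with delayed loops, handing each its path.
; EnemyKilled decrements the enemy count, updating the HUD or switching round type at zero.
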(event `self.ReceiveBeginPlay`
  (bind _asbp_player_controller (cast `/Game/GameJamGame/Blueprints/BP_PlayerController` (`GameplayStatics.GetPlayerController` 0)))
  (`self.SpawnInitialRooms` _asbp_player_controller))

(event `StartWave`
  (bind _outactors (`GameplayStatics.GetAllActorsOfClass` "/Game/GameJamGame/Blueprints/Rooms/BP_Room.BP_Room_C"))
  (for _array_element _outactors
    (`/Game/GameJamGame/Blueprints/Rooms/BP_Room.SetPathfindingValues` _array_element))
  (bind _returnvalue (`GameplayStatics.GetActorOfClass` "/Game/BP_PathFinding.BP_PathFinding_C"))
  (bind _output_get (set `self.PathFind` _returnvalue))
  (bind _haspath (`/Game/BP_PathFinding.HasPathToGoal` _output_get (`/Game/GameJamGame/Blueprints/Rooms/BP_Room.BP_PathFindingNode` (cast `/Game/GameJamGame/Blueprints/Rooms/BP_Room` (`self.EnemySpawnTile`) :!pure true)) (`/Game/GameJamGame/Blueprints/Rooms/BP_Room.BP_PathFindingNode` (cast `/Game/GameJamGame/Blueprints/Rooms/BP_Room` (`self.TreasureTile`) :!pure true))))
  (if _haspath
    (`self.SetEnemyPath`)
    (set `self.RoundType` "NewEnumerator0")
    (bind _result (`/Engine/EditorBlueprintResources/StandardMacros.IncrementInt` (`self.CurrentWaveNumber`))
      (:`  `
        (bind _returnvalue_2 (`|GetDataTableRow` "/Game/GameJamGame/Blueprints/Structs_and_DTs/DT_Waves.DT_Waves" (`KismetStringLibrary.Conv_StringToName` (`KismetStringLibrary.Conv_IntToString` _result)))
          (:`then`
            (`self.SpawnEnemy` (break `/Game/GameJamGame/Blueprints/Structs_and_DTs/S_WaveSpawner` _returnvalue_2) (`.WalkerAmount_23_E0BB4E064343876586A32B9606C6CBCF` (break `/Game/GameJamGame/Blueprints/Structs_and_DTs/S_WaveSpawner` _returnvalue_2)) (`.WalkerSpawnDelay_22_F44385EE4613DB28911F4788F7ECBA74` (break `/Game/GameJamGame/Blueprints/Structs_and_DTs/S_WaveSpawner` _returnvalue_2)) ; Spawn Walker
              (:`__`
                (`self.SpawnEnemy` (`.FlyerBP_28_5F166F2A4918EDBF073B41ACB921BA99` (break `/Game/GameJamGame/Blueprints/Structs_and_DTs/S_WaveSpawner` _returnvalue_2)) (`.FlyerAmount_20_8BDDC3E54B52099061A253BBCC6692B5` (break `/Game/GameJamGame/Blueprints/Structs_and_DTs/S_WaveSpawner` _returnvalue_2)) (`.FlyerSpawnDelay_21_6427CED34282917F07D826865784EF9E` (break `/Game/GameJamGame/Blueprints/Structs_and_DTs/S_WaveSpawner` _returnvalue_2)) ; Spawn Flyer
                  (:`__`
                    (set `self.CurrentEnemyCount` (+ (`.WalkerAmount_23_E0BB4E064343876586A32B9606C6CBCF` (break `/Game/GameJamGame/Blueprints/Structs_and_DTs/S_WaveSpawner` _returnvalue_2)) (`.FlyerAmount_20_8BDDC3E54B52099061A253BBCC6692B5` (break `/Game/GameJamGame/Blueprints/Structs_and_DTs/S_WaveSpawner` _returnvalue_2))))))))))))
    (else
      (`KismetSystemLibrary.PrintString` "NO PATH" true true (struct :`R` 1.0 :`G` 0.033106 :`A` 1.0) 20.0))))

(event `EnemyKilled`
  (bind _output_get (set `self.CurrentEnemyCount` (- (`self.CurrentEnemyCount`) 1)))
  (if (== _output_get 0)
    (`self.WaveEnd`)
    (else
      (`self.UpdateEnemyCountHUDText`))))

(event `WaveEnd`
  (set `self.RoundType` "NewEnumerator1"))

(fn `SetEnemyPath`
  (bind (_finalpath _foundpath) (`/Game/BP_PathFinding.FindPath` (`self.PathFind`) (`/Game/GameJamGame/Blueprints/Rooms/BP_Room.BP_PathFindingNode` (cast `/Game/GameJamGame/Blueprints/Rooms/BP_Room` (`self.EnemySpawnTile`) :!pure true)) (`/Game/GameJamGame/Blueprints/Rooms/BP_Room.BP_PathFindingNode` (cast `/Game/GameJamGame/Blueprints/Rooms/BP_Room` (`self.TreasureTile`) :!pure true)) "Walker"))
  (set `self.WalkerPath` _finalpath)
  (`KismetSystemLibrary.PrintString` (`KismetStringLibrary.Conv_BoolToString` _foundpath) true true (struct :`R` 1.0 :`G` 0.291246 :`A` 1.0))
  (bind _finalpath_2 (`/Game/BP_PathFinding.FindPath` (`self.PathFind`) (`/Game/GameJamGame/Blueprints/Rooms/BP_Room.BP_PathFindingNode` (cast `/Game/GameJamGame/Blueprints/Rooms/BP_Room` (`self.EnemySpawnTile`) :!pure true)) (`/Game/GameJamGame/Blueprints/Rooms/BP_Room.BP_PathFindingNode` (cast `/Game/GameJamGame/Blueprints/Rooms/BP_Room` (`self.TreasureTile`) :!pure true)) "Flyer"))
  (set `self.FlyerPath` _finalpath_2))

(fn `SpawnInitialRooms`
  (params (`Player Controller` :type "/Game/GameJamGame/Blueprints/BP_PlayerController Object Reference"))
  (set `/Game/GameJamGame/Blueprints/BP_PlayerController.CurrentlyRoomBuilt` 6 `Player Controller`)
  (set `/Game/GameJamGame/Blueprints/BP_PlayerController.SelectedGridSpot` (-500.0 0.0 0.0) `Player Controller`)
  (bind _actor_spawned (`/Game/GameJamGame/Blueprints/BP_PlayerController.SpawnRoom` `Player Controller` false))
  (set `self.EnemySpawnTile` _actor_spawned)
  (set `/Game/GameJamGame/Blueprints/BP_PlayerController.SelectedGridSpot` (-300.0 0.0 0.0) `Player Controller`)
  (set `/Game/GameJamGame/Blueprints/BP_PlayerController.CurrentlyRoomBuilt` 5 `Player Controller`)
  (bind _actor_spawned_2 (`/Game/GameJamGame/Blueprints/BP_PlayerController.SpawnRoom` `Player Controller` false))
  (set `self.TreasureTile` _actor_spawned_2)
  (set `/Game/GameJamGame/Blueprints/BP_PlayerController.CurrentlyRoomBuilt` 2 `Player Controller`))

(fn `UpdateEnemyCountHUDText`
  (`/Game/GameJamGame/TudorDev/W_PlayerHUD.Update_Enemy_Text` (`self.As W Player HUD`) (`self.CurrentEnemyCount`)))

(fn `UpdateWaveCountHUDText`
  (`/Game/GameJamGame/TudorDev/W_PlayerHUD.Update_Wave_Text` (`self.As W Player HUD`) (`self.CurrentWaveNumber`) 0))

(fn `UserConstructionScript`)