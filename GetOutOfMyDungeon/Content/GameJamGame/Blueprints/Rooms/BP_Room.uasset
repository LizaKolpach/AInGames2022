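; BP_Room is a grid-placed room actor that supports a translucent ghost state and can replace itself with another room class.
; BeginPlay and ToggleGhost set sprite opacity through a dynamic material and hand the room reference to its build-button widget.
; For non-ghost rooms, SetPathfindingValues derives node coordinates from the player controller's grid size and links adjacent rooms' pathfinding nodes, using fixed four-way offsets.
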(event `RoomChange2`
  (params (RoomToChangeTo :type "/Game/GameJamGame/Blueprints/Rooms/BP_Room Class Reference"))
  (`|SpawnActorFromClass` RoomToChangeTo (`self.GetTransform`) "Undefined" "OverrideRootScale" null (`self.GridLocation`) false null)
  (`self.K2_DestroyActor`))

(event `ToggleGhost`
  (params (IsGhost :type Boolean))
  (bind _returnvalue (`WidgetComponent.GetWidget` (`self.BuildButtonWidget`)))
  (set `self.IsGhost` IsGhost)
  (if (`self.IsGhost`) :!label _label
    ;[1 1 1] Set opacity of the material
    (set `self.Opacity` 0.5)
    (else
      (set `self.Opacity` 1.0)))
  (bind _returnvalue_2 (`KismetMaterialLibrary.CreateDynamicMaterialInstance` (`PrimitiveComponent.GetMaterial` (`self.RoomBase`) 0)))
  (bind _output_get (set `self.SpriteMaterial` _returnvalue_2))
  (`MaterialInstanceDynamic.SetScalarParameterValue` _output_get "Opacity" (`self.Opacity`))
  (`PrimitiveComponent.SetMaterial` (`self.RoomBase`) 0 (`self.SpriteMaterial`))
  ;[1 1 1] Set reference of self to widgets
  (set `self.HazardMenuButtonRef` _returnvalue)
  (set `/Game/GameJamGame/Blueprints/WBP_BuildRoomButton.RoomRef` self (cast `/Game/GameJamGame/Blueprints/WBP_BuildRoomButton` _returnvalue :!pure true)))

(event `ToggleWidgetVisibility`
  (params (`New Visibility` :type Boolean))
  (`SceneComponent.SetVisibility` (`self.BuildButtonWidget`) `New Visibility` false))

(event `self.ReceiveBeginPlay`
  (`|ExecutionSequence`
    (:`then_0`
      (goto _label))))

(event `SetPathfindingValues`
  (bind _gridlocation (`self.GridLocation`))
  (if (not (`self.IsGhost`))
    (`self.SetPathfindingGridLocation`)
    (`KismetArrayLibrary.Array_Clear` (`/Game/BP_PathFindingNode.Neighbours` (`self.BP_PathFindingNode`)))
    (`self.SetNeighbours` (+ _gridlocation (100.0 0.0 0.0)))
    (`self.SetNeighbours` (+ _gridlocation (-100.0 0.0 0.0)))
    (`self.SetNeighbours` (+ _gridlocation (0.0 100.0 0.0)))
    (`self.SetNeighbours` (+ _gridlocation (0.0 -100.0 0.0)))))

(fn `SetNeighbours`
  (params (GridPosition :type "Vector Structure"))
  (bind _value (`/Game/GameJamGame/Blueprints/BP_PlayerController.GetRoomAtSelectedGridPosition` (`self.As BP Player Controller`) GridPosition))
  (`/Engine/EditorBlueprintResources/StandardMacros.IsValid` _value
    (:`Is Valid`
      (bind _asbp_room (cast `/Game/GameJamGame/Blueprints/Rooms/BP_Room` _value))
      (`KismetArrayLibrary.Array_Add` (`/Game/BP_PathFindingNode.Neighbours` (`self.BP_PathFindingNode`)) (`/Game/GameJamGame/Blueprints/Rooms/BP_Room.BP_PathFindingNode` _asbp_room)))))

(fn `SetPathfindingGridLocation`
  (bind _bp_pathfindingnode (`self.BP_PathFindingNode`))
  (bind (_gridlocation_x _gridlocation_y) (`KismetMathLibrary.BreakVector` (`self.GridLocation`)))
  (bind _asbp_player_controller (cast `/Game/GameJamGame/Blueprints/BP_PlayerController` (`GameplayStatics.GetPlayerController` 0)))
  (bind _output_get (set `self.As BP Player Controller` _asbp_player_controller))
  (bind _gridsize (`/Game/GameJamGame/Blueprints/BP_PlayerController.GridSize` _output_get))
  (bind _output_get_2 (set `/Game/BP_PathFindingNode.GridPositionX` (`KismetMathLibrary.FTrunc` (/ _gridlocation_x _gridsize)) _bp_pathfindingnode))
  (bind _output_get_3 (set `/Game/BP_PathFindingNode.GridPositionY` (`KismetMathLibrary.FTrunc` (/ _gridlocation_y _gridsize)) _bp_pathfindingnode))
  (`KismetSystemLibrary.PrintString` (`KismetStringLibrary.Concat_StrStr` "x: " (`KismetStringLibrary.Conv_IntToString` _output_get_2) "y: " (`KismetStringLibrary.Conv_IntToString` _output_get_3))))

(fn `UserConstructionScript`)