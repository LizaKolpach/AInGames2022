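; Player controller for a dungeon game that switches between Build and Battle modes held in the game mode.
; In Build mode, Tick snaps the cursor hit to a grid and respawns a ghost room preview when the cell changes.
; Clicks place, pick up and move, or destroy rooms tracked in a location-to-actor map.
; In Battle mode, clicks line-trace to damage enemies; test keys switch mode and room type.
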(event `self.ReceiveBeginPlay`
  (bind _asgm_dungeon_game_mode (cast `/Game/GameJamGame/Blueprints/GM_DungeonGameMode` (`GameplayStatics.GetGameMode`)))
  (set `self.As GM Dungeon Game Mode` _asgm_dungeon_game_mode))

(event `NewGridSpotSelected`
  (params (GridLocation :type "Vector Structure"))
  (bind _ghost_spawned (`self.Ghost Spawned`))
  ;[1 1 1] Destroy and spawn a new ghost on the new grid spot
  (`/Engine/EditorBlueprintResources/StandardMacros.IsValid` _ghost_spawned
    (:`Is Valid`
      (`self.K2_DestroyActor` _ghost_spawned))
    (:`Is Not Valid`
      _))
  (if (not (`self.IsSelectedGridPositionOccupied`))
    (bind _actor_spawned (`self.SpawnRoom` true))
    (set `self.Ghost Spawned` _actor_spawned)))

(event `self.ReceiveTick`
  (params (DeltaSeconds :type "Float (single-precision)"))
  (bind _returnvalue (/ (`self.GridSize`) 2.0))
  (switch `/Game/GameJamGame/Blueprints/eRoundType` (`/Game/GameJamGame/Blueprints/GM_DungeonGameMode.RoundType` (`self.As GM Dungeon Game Mode`))
    (:`NewEnumerator1`
      (`self.CheckNewGridSpotSelected`)
      (`|ExecutionSequence`
        (:`then_0`
          (if (`self.HasRoomSelected`)
            ;[1 1 1] Selecting a room to move
            (bind _asbp_room (cast `/Game/GameJamGame/Blueprints/Rooms/BP_Room` (`self.SelectedRoom`)))
            (`/Game/GameJamGame/Blueprints/Rooms/BP_Room.ToggleGhost` _asbp_room false)
            (`BlueprintMapLibrary.Map_Remove` (`self.GridSlots`) (`self.K2_GetActorLocation` _asbp_room))
            (`self.K2_SetActorLocation` _asbp_room (`self.SelectedGridSpot`) false false)))
        (:`then_2`
          ;[1 0 0] DEBUG TESTING
          (`KismetSystemLibrary.DrawDebugBox` (`self.SelectedGridSpot`) (`KismetMathLibrary.MakeVector` _returnvalue _returnvalue) (struct :`R` 1.0 :`G` 0.084869 :`A` 1.0) (struct) 0.0 5.0))))))

(event `Key|Two`
  (params (Key :type "Key Structure"))
  ;[1 0 0] TEST - changing types of rooms
  (:`Pressed`
    (set `self.CurrentlyRoomBuilt` 2)))

(event `Key|Three`
  (params (Key :type "Key Structure"))
  ;[1 0 0] TEST - changing types of rooms
  (:`Pressed`
    (set `self.CurrentlyRoomBuilt` 3)))

(event `Key|Four`
  (params (Key :type "Key Structure"))
  ;[1 0 0] TEST - changing types of rooms
  (:`Pressed`
    (set `self.CurrentlyRoomBuilt` 4)))

(event `Key|One`
  (params (Key :type "Key Structure"))
  (bind _as_gm_dungeon_game_mode (`self.As GM Dungeon Game Mode`))
  (:`Pressed`
    ;[1 0 0] DEBUG TESTING
    ;;[1 1 1] changing between battle and build mode
    (switch `/Game/GameJamGame/Blueprints/eRoundType` (`/Game/GameJamGame/Blueprints/GM_DungeonGameMode.RoundType` (`self.As GM Dungeon Game Mode`))
      (:`NewEnumerator0`
        (set `/Game/GameJamGame/Blueprints/GM_DungeonGameMode.RoundType` "NewEnumerator1" _as_gm_dungeon_game_mode)
        (`KismetSystemLibrary.PrintString` "BuildMode"))
      (:`NewEnumerator1`
        (set `/Game/GameJamGame/Blueprints/GM_DungeonGameMode.RoundType` "NewEnumerator0" _as_gm_dungeon_game_mode)
        (`KismetSystemLibrary.PrintString` "BattleMode")))))

(event `InputAction|Click`
  (params (Key :type "Key Structure"))
  (bind (_worldlocation _worlddirection) (`self.DeprojectMousePositionToWorld`))
  (bind _selectedroom (`self.SelectedRoom`))
  (:`Pressed`
    (switch `/Game/GameJamGame/Blueprints/eRoundType` (`/Game/GameJamGame/Blueprints/GM_DungeonGameMode.RoundType` (`self.As GM Dungeon Game Mode`))
      (:`NewEnumerator0`
        ;[1 1 1] ApplyDamage to BP_Enemy
        (bind _outhit (`KismetSystemLibrary.LineTraceSingle` _worldlocation (+ _worldlocation (* _worlddirection 1000.0)) "TraceTypeQuery1"))
        (bind _asbp_enemy (cast `/Game/GameJamGame/Enemies/BP_Enemy` (`.HitActor` (`GameplayStatics.BreakHitResult` _outhit))))
        (`GameplayStatics.ApplyDamage` _asbp_enemy (`self.BaseClickDamage`)))
      (:`NewEnumerator1`
        ;[1 1 1] Place a room on a grid cell
        (if (`self.IsSelectedGridPositionOccupied`)
          (if (not (`self.HasRoomSelected`))
            (set `self.SelectedRoom` (`self.GetRoomAtSelectedGridPosition`))
            (set `self.HasRoomSelected` true))
          (elif (`self.HasRoomSelected`)
            (bind _asbp_room (cast `/Game/GameJamGame/Blueprints/Rooms/BP_Room` _selectedroom))
            (`/Game/GameJamGame/Blueprints/Rooms/BP_Room.ToggleGhost` _asbp_room false)
            (`BlueprintMapLibrary.Map_Add` (`self.GridSlots`) (`self.SelectedGridSpot`) _selectedroom)
            (set `self.SelectedRoom` null)
            (set `self.HasRoomSelected` false)
            (else
              (`self.SpawnRoom` false))))))))

(event `InputAction|RightClick`
  (params (Key :type "Key Structure"))
  ;[1 1 1] Destroy a room
  (:`Pressed`
    (switch `/Game/GameJamGame/Blueprints/eRoundType` (`/Game/GameJamGame/Blueprints/GM_DungeonGameMode.RoundType` (`self.As GM Dungeon Game Mode`))
      (:`NewEnumerator1`
        (if (`self.IsSelectedGridPositionOccupied`)
          (`self.K2_DestroyActor` (`self.GetRoomAtSelectedGridPosition`))
          (`BlueprintMapLibrary.Map_Remove` (`self.GridSlots`) (`self.SelectedGridSpot`)))))))

(fn `CheckNewGridSpotSelected`
  (bind _gridposition (`self.Get Grid Position`))
  (bind _output_get (set `self.SelectedGridSpot` _gridposition))
  (if (not (`KismetMathLibrary.EqualExactly_VectorVector` _output_get (`self.PreviousSelectedGridspot`)))
    (bind _output_get_2 (set `self.SelectedGridSpot` _gridposition))
    (bind _output_get_3 (set `self.PreviousSelectedGridspot` _output_get_2))
    (`self.NewGridSpotSelected` _output_get_3)))

(fn `Get Grid Position`
  (returns (GridPosition :type "Vector Structure"))
  (bind (_returnvalue_x _returnvalue_y) (`KismetMathLibrary.BreakVector` (`KismetMathLibrary.Vector_SnappedToGrid` (`.ImpactPoint` (`GameplayStatics.BreakHitResult` (`self.GetHitResultUnderCursorByChannel` "TraceTypeQuery2"))) (`self.GridSize`))))
  (return (`KismetMathLibrary.MakeVector` _returnvalue_x _returnvalue_y)))

(fn `GetRoomAtSelectedGridPosition`
  (returns (Value :type "Actor Object Reference"))
  (return (`BlueprintMapLibrary.Map_Find` (`self.GridSlots`) (`self.SelectedGridSpot`))))

(fn `IsSelectedGridPositionOccupied`
  (returns (ReturnValue :type Boolean))
  (return (`BlueprintMapLibrary.Map_Contains` (`self.GridSlots`) (`self.SelectedGridSpot`))))

(fn `SpawnRoom`
  (params (IsGhost :type Boolean))
  (returns (`Actor Spawned` :type "Actor Object Reference"))
  (bind _selectedgridspot (`self.SelectedGridSpot`))
  (bind _returnvalue (`|SpawnActorFromClass` (`BlueprintMapLibrary.Map_Find` (`self.RoomTypes`) (`self.CurrentlyRoomBuilt`)) (`KismetMathLibrary.MakeTransform` _selectedgridspot (struct) (`KismetMathLibrary.Conv_DoubleToVector` (/ (`self.GridSize`) 100.0))) "AlwaysSpawn" "OverrideRootScale" null _selectedgridspot IsGhost null))
  (if IsGhost
    (return _returnvalue)
    (else
      (`BlueprintMapLibrary.Map_Add` (`self.GridSlots`) (`self.K2_GetActorLocation` _returnvalue) _returnvalue)
      (return _returnvalue))))

(fn `UserConstructionScript`)