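; BP_AudioManager handles screen-based background music, starting the "Main" track on BeginPlay.
; SwitchMusic looks up the screen name in the ScreensToMusic map and compares the result directly to the CurrentMusic audio component.
; When they differ, it pauses the current component and StartNewMusic creates and plays a new 2D sound from the beginning.
; Previous components are only paused, never stopped or resumed here.
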(event `self.ReceiveBeginPlay`
  (`self.SwitchMusic` "Main"))

(event `SwitchMusic`
  (params (ScreenName :type Name))
  (set `self.ScreenName` ScreenName)
  (`/Engine/EditorBlueprintResources/StandardMacros.IsValid` (`self.CurrentMusic`)
    (:`Is Valid`
      (if (not (== (`BlueprintMapLibrary.Map_Find` (`self.ScreensToMusic`) (`self.ScreenName`)) (`self.CurrentMusic`)))
        (`AudioComponent.SetPaused` (`self.CurrentMusic`) true)
        (`self.StartNewMusic`)))
    (:`Is Not Valid`
      (`self.StartNewMusic`))))

(event `StartNewMusic`
  (bind _returnvalue (`GameplayStatics.CreateSound2D` (`BlueprintMapLibrary.Map_Find` (`self.ScreensToMusic`) (`self.ScreenName`)) 1.0 1.0 0.0 null))
  (bind _output_get (set `self.CurrentMusic` _returnvalue))
  (`AudioComponent.Play` _output_get 0.0))

(fn `UserConstructionScript`)